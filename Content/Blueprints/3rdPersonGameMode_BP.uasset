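; Third-person game mode that runs a countdown timer and ends the game when it runs out.
; Tick feeds a one-second Delay, which throttles the decrement of Seconds to roughly once per second.
; At zero it prints a game over message, spawns a GameOver actor at the player character's transform, then pauses the game after a short delay.
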(event `self.ReceiveTick`
  (params (DeltaSeconds :type "Float (single-precision)"))
  (bind _seconds (`self.Seconds`))
  ;[1 1 1] Allows the time to be connected to the player so when it is over something happens
  (`KismetSystemLibrary.Delay` 1.0)
  (if (> _seconds 0)
    (set `self.Seconds` (- _seconds 1))
    (else
      ;;[1 0.009844 0] If false game over
      (`KismetSystemLibrary.PrintString` "Game Over")
      ;[1 0.2036 0] This will spawn the game over actor over the players head
      (`|SpawnActorFromClass` "/Game/Blueprints/GameOver.GameOver_C" (`self.GetTransform` (`GameplayStatics.GetPlayerCharacter` 0)) "Undefined" "OverrideRootScale" null null)
      (`KismetSystemLibrary.Delay` 1.0)
      (`GameplayStatics.SetGamePaused` true))))

(fn `UserConstructionScript`)