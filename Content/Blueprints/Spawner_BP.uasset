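; Spawner blueprint that places Pickup_BP actors one at a time at a sequence of locations.
; BeginPlay spawns a pickup at the transform of the current entry in the Pickups actor array.
; The NextPickup event advances the Current index, wraps to the first entry past the end, and spawns the next pickup there.
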(event `self.ReceiveBeginPlay`
  ;[1 1 1] Creates the spawn array for the pickups
  ;;[0.2282 0.2508 1] spawns the PickUp BP in
  (`|SpawnActorFromClass` "/Game/Blueprints/Pickup_BP.Pickup_BP_C" (`self.GetTransform` (`|GetArrayItem` (`self.Pickups`) (`self.Current`))) "Undefined" "OverrideRootScale" null null :!label _label))

(event `NextPickup`
  ;[1 1 1] Creates the spawn array for the pickups
  ;;[1 0.2896 0.2598] Sets up function for next pickup
  (bind _result (`/Engine/EditorBlueprintResources/StandardMacros.IncrementInt` (`self.Current`))
    (:`  `
      (if (< _result (`KismetArrayLibrary.Array_Length` (`self.Pickups`)))
        (goto _label)
        (else
          (set `self.Current` 0)
          (goto _label))))))

(fn `UserConstructionScript`)